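; Player-controlled bowling ball that is launched by a physics impulse and steered by rotating its velocity.
; Tick polls the GameInstance's pin-knocked flag, then writes the score to the frame UI by throw number, advancing the frame after the second throw.
; Respawn stops the ball, moves it to the PlayerStart indexed by current frame and has pins delete knocked ones.
; The low-speed respawn and throw-counter reset logic are disconnected.
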(event `self.ReceiveTick`
  (params (DeltaSeconds :type "Float (single-precision)"))
  (bind _gameinstance (`self.GameInstance`))
  (bind _gameinstance_2 (`self.GameInstance`))
  (bind _returnvalue (`KismetTextLibrary.Conv_IntToText` (`/Game/Blueprints/BP_GameInstance.Score` (`self.GameInstance`))))
  ;[1 0 0] Event Tick
  ;[1 1 1] Check if pin has been knocked over
  (if (`/Game/Blueprints/BP_GameInstance.PinKnockedOver` _gameinstance_2)
    (set `/Game/Blueprints/BP_GameInstance.PinKnockedOver` false _gameinstance_2)
    ;[1 1 1] After Throw
    (switch `int` (`/Game/Blueprints/BP_GameInstance.ThrowNumber` (`self.GameInstance`))
      (:`Default`
        ;;[1 1 1] First Throw
        (`/Game/Blueprints/WB_Frame.SetTextBlocks` (`/Game/Blueprints/WB_GameUI.WB_Frame` (`self.Game UI`)) (`KismetTextLibrary.Conv_IntToText` (`/Game/Blueprints/BP_GameInstance.Score` (`self.GameInstance`))) "" "" :!label _label)
        (`self.Respawn`)
        (set `/Game/Blueprints/BP_GameInstance.ThrowNumber` 1 (`self.GameInstance`)))
      (:`1`
        (goto _label))
      (:`2`
        ;;[1 1 1] After Second Throw
        (`/Game/Blueprints/WB_Frame.SetTextBlocks` (`/Game/Blueprints/WB_GameUI.WB_Frame` (`self.Game UI`)) "" _returnvalue _returnvalue)
        (set `/Game/Blueprints/BP_GameInstance.CurrentFrame` (+ (`/Game/Blueprints/BP_GameInstance.CurrentFrame` _gameinstance) 1) _gameinstance)
        (`self.Respawn`)))))

(event `self.ReceiveBeginPlay`
  ;[1 0 0] Event BeginPlay
  ;[1 1 1] Input Mapping
  (`EnhancedInputSubsystemInterface.AddMappingContext` (pcsubsystem `EnhancedInputLocalPlayerSubsystem` (`GameplayStatics.GetPlayerController` 0)) "/Game/Input/IMC_Default.IMC_Default" 0 (struct))
  ;[1 1 1] Comment
  (bind _returnvalue (`|CreateWidget` "/Game/Blueprints/WB_GameUI.WB_GameUI_C"))
  (bind _output_get (set `self.Game UI` _returnvalue))
  (`UserWidget.AddToViewport` _output_get 0)
  (bind _asbp_game_instance (cast `/Game/Blueprints/BP_GameInstance` (`GameplayStatics.GetGameInstance`)))
  (set `self.GameInstance` _asbp_game_instance)
  (`self.Respawn`))

(event `EnhancedInput|/Game/Input/LaunchSphere`
  (params (ActionValue :type Boolean) (ElapsedSeconds :type "Float (double-precision)") (TriggeredSeconds :type "Float (double-precision)") (InputAction :type "InputAction Object Reference" :default "/Game/Input/LaunchSphere.LaunchSphere"))
  (bind _gameinstance (`self.GameInstance`))
  ;[1 1 1] Launch Ball
  (:`Triggered`
    (if (not (`self.IsRolling`))
      (set `self.IsRolling` true)
      (`PrimitiveComponent.AddImpulse` (`self.Sphere`) (* (`self.GetActorForwardVector`) (200000.0 0.0 0.0)) "None" false)
      (set `/Game/Blueprints/BP_GameInstance.ThrowNumber` (+ (`/Game/Blueprints/BP_GameInstance.ThrowNumber` _gameinstance) 1) _gameinstance))))

(event `EnhancedInput|/Game/Input/MoveRight`
  (params (ActionValue :type "Float (double-precision)") (ElapsedSeconds :type "Float (double-precision)") (TriggeredSeconds :type "Float (double-precision)") (InputAction :type "InputAction Object Reference" :default "/Game/Input/MoveRight.MoveRight"))
  ;[1 1 1] Rotation
  (:`Triggered`
    (bind _returnvalue (`PrimitiveComponent.GetPhysicsLinearVelocity` (`self.Sphere`) "None"))
    (`PrimitiveComponent.SetPhysicsLinearVelocity` (`self.Sphere`) (`KismetMathLibrary.GreaterGreater_VectorRotator` _returnvalue (`KismetMathLibrary.MakeRotator` 0.0 0.0 (* ActionValue 1.0))) false "None")))

(fn `Respawn`
  (set `self.IsRolling` false)
  (`KismetSystemLibrary.PrintString` "Respawn")
  ;[1 1 1] Set Ball position/rotation/velocity
  (bind _outactors (`GameplayStatics.GetAllActorsOfClass` "/Script/Engine.PlayerStart"))
  (bind _output (`|GetArrayItem` _outactors (`/Game/Blueprints/BP_GameInstance.CurrentFrame` (`self.GameInstance`))))
  (`KismetSystemLibrary.PrintString` (`KismetSystemLibrary.GetDisplayName` _output))
  (`self.K2_SetActorLocationAndRotation` (`self.K2_GetActorLocation` _output) (`self.K2_GetActorRotation` _output))
  (`PrimitiveComponent.SetPhysicsLinearVelocity` (`self.Sphere`) (0.0 0.0 0.0) false "None")
  (`PrimitiveComponent.SetPhysicsAngularVelocityInRadians` (`self.Sphere`) (0.0 0.0 0.0) false "None")
  ;[1 1 1] Remove Knocked over pins
  (bind _outactors_2 (`GameplayStatics.GetAllActorsOfClass` "/Game/Blueprints/BP_Pin.BP_Pin_C"))
  (for _array_element _outactors_2
    (`/Game/Blueprints/BP_Pin.Delete Knocked Pins` _array_element)))

(fn `UserConstructionScript`)