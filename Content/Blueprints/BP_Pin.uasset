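; BP_Pin is a pin actor that detects when it has been knocked over and scores it.
; Each Tick it checks whether roll or pitch exceeds a tilt threshold, latching IsKnockedOver so it counts only once.
; On falling it restarts the timer in BP_GameInstance, increments the shared score there and prints it.
; A separate DeleteKnockedPins function destroys the pin if it has fallen.
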(event `self.ReceiveTick`
  (params (DeltaSeconds :type "Float (single-precision)"))
  (bind (_returnvalue_roll _returnvalue_pitch) (`KismetMathLibrary.BreakRotator` (`self.K2_GetActorRotation`)))
  ;[1 1 1] Check if pin is upright
  (if (`self.isKnockedOver`)
    _
    (elif (or (> (`KismetMathLibrary.Abs` _returnvalue_roll) 45.0) (> (`KismetMathLibrary.Abs` _returnvalue_pitch) 45.0))
      (set `self.isKnockedOver` true)
      (bind _asbp_game_instance (cast `/Game/Blueprints/BP_GameInstance` (`GameplayStatics.GetGameInstance`)))
      (`/Game/Blueprints/BP_GameInstance.RestartTimer` _asbp_game_instance)
      (bind _output_get (set `/Game/Blueprints/BP_GameInstance.Score` (+ (`/Game/Blueprints/BP_GameInstance.Score` _asbp_game_instance) 1) _asbp_game_instance))
      (`KismetSystemLibrary.PrintString` (`KismetStringLibrary.Conv_IntToString` _output_get)))))

(fn `Delete Knocked Pins`
  (if (`self.isKnockedOver`)
    (`self.K2_DestroyActor`)))

(fn `UserConstructionScript`)